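; SmokingPipe_BP is a Level 2 pipe actor that releases smoke the first time it takes damage.
; AnyDamage passes through a DoOnce into the Explode event, so it triggers only once.
; Explode activates the Smoke and BPHiddenVolume components, plays a click sound at the actor and enlarges the hidden volume to a fixed scale.
; It also prints a leftover debug string.
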(event `self.ReceiveAnyDamage`
  (params (Damage :type "Float (single-precision)") (DamageType :type "DamageType Object Reference") (InstigatedBy :type "Controller Object Reference") (DamageCauser :type "Actor Object Reference"))
  (`/Engine/EditorBlueprintResources/StandardMacros.DoOnce` false
    (:`Completed`
      (`self.Explode`))))

(event `Explode`
  (`ActorComponent.Activate` (`self.Smoke`) false)
  (`ActorComponent.Activate` (`self.BP_HiddenVolume`) false)
  (`GameplayStatics.PlaySoundAtLocation` "/Game/AdvancedLocomotionV4/Audio/UI/Click.Click" (`self.K2_GetActorLocation`) (struct) 1.0 1.0 0.0 null null null null)
  (`SceneComponent.SetRelativeScale3D` (`self.BP_HiddenVolume`) (16.0 17.0 20.0))
  (`KismetSystemLibrary.PrintString` "Hello"))

(fn `UserConstructionScript`)