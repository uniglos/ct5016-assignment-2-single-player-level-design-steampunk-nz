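; Exploding pipe actor in Level 2 that blows up the first time it takes any damage.
; AnyDamage passes through a DoOnce into Explode, which plays smoke briefly, then hides the mesh and smoke.
; It then applies full radial damage around itself and fires a radial force impulse.
; Debug prints mark each stage, and the actor is hidden rather than destroyed.
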(event `Explode`
  (`KismetSystemLibrary.PrintString` "hit")
  (`ActorComponent.Activate` (`self.Smoke`) false)
  (`KismetSystemLibrary.PrintString` "Smoke")
  (`KismetSystemLibrary.Delay` 1.5)
  (`ActorComponent.Deactivate` (`self.Smoke`))
  (`SceneComponent.SetHiddenInGame` (`self.StaticMesh`) true false)
  (`SceneComponent.SetHiddenInGame` (`self.Smoke`) true false)
  (`KismetSystemLibrary.PrintString` "hidden")
  (`GameplayStatics.ApplyRadialDamage` :`BaseDamage` 50.0 :`Origin` (`self.K2_GetActorLocation`) :`DamageRadius` 50.0 :`DamageCauser` null :`InstigatedByController` null :`bDoFullDamage` true)
  (`KismetSystemLibrary.PrintString` "Damage")
  (`RadialForceComponent.FireImpulse` (`self.RadialForce`))
  (`KismetSystemLibrary.PrintString` "boom"))

(event `self.ReceiveAnyDamage`
  (params (Damage :type "Float (single-precision)") (DamageType :type "DamageType Object Reference") (InstigatedBy :type "Controller Object Reference") (DamageCauser :type "Actor Object Reference"))
  (`/Engine/EditorBlueprintResources/StandardMacros.DoOnce` false
    (:`Completed`
      (`self.Explode`))))

(fn `UserConstructionScript`)